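; BP_BossEvents is a placeable one-shot trigger that scripts the zombie boss's behavior when the player enters its box.
; On overlap it teleports BP_Boss to a raised teleport point, optionally plays a cinematic, then destroys itself.
; Optional flags write a patrol override and a timed wait to the boss's Blackboard, whose reference is cached only in the patrol branch.
; The Construction Script sizes the box and previews the teleport point with debug line and label.
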(event OnComponentBeginOverlap(BoxCollision)
  (params (OverlappedComponent :type Primitive%20Component%20Object%20Reference) (OtherActor :type Actor%20Object%20Reference) (OtherComp :type Primitive%20Component%20Object%20Reference) (OtherBodyIndex :type Integer) (bFromSweep :type Boolean) (SweepResult :type Hit%20Result%20Structure%20%28by%20ref%29))
  (if (Actor|ActorHasTag OtherActor "Player")
    (bind _returnvalue (Actor|GetActorOfClass "/Game/AI_Zombie/BP_Boss.BP_Boss_C"))
    (bind _output_get (Variables|Default|SetRefBoss _returnvalue))
    (Transformation|SetActorLocation _output_get (+ (Transformation|GetWorldLocation (Variables|Default|GetTeleportpoint)) "0.000000,0.000000,110.000000") false false)
    (if (Variables|Default|GetbNeedCinematic?)
      (Sequencer|Player|Play (Variables|/Script/LevelSequence.LevelSequenceActor|GetSequencePlayer (Variables|Default|GetCinematicToPlay)) :!class /Script/MovieScene.MovieSceneSequencePlayer))
    (if (Variables|Default|GetbSetupPatrolPoint?)
      (Variables|Default|SetBlackboardBoss (AI|GetBlackboard (AI|GetAIController (Variables|Default|GetRefBoss))))
      (AI|Components|Blackboard|SetValueasVector (Variables|Default|GetBlackboardBoss) (Utilities|Name|MakeLiteralName "TargetLocation") (Transformation|GetActorLocation (Variables|Default|GetPatrolPoint)))
      (AI|Components|Blackboard|SetValueasBool (Variables|Default|GetBlackboardBoss) (Utilities|Name|MakeLiteralName "IsOverrided") true))
    (if (Variables|Default|GetbShouldWait?)
      (AI|Components|Blackboard|SetValueasBool (Variables|Default|GetBlackboardBoss) (Utilities|Name|MakeLiteralName "ShouldWait") true)
      (AI|Components|Blackboard|SetValueasFloat (Variables|Default|GetBlackboardBoss) (Utilities|Name|MakeLiteralName "WaitingTime") (Variables|Default|GetWaitingTime)))
    (Actor|DestroyActor)))

(fn ConstructionScript
  (Components|Box|SetBoxExtent (Variables|Default|GetBoxCollision) (Variables|Default|GetColliderSize) true)
  (Transformation|SetRelativeLocation (Variables|Default|GetTeleportpoint) (Variables|Default|GetTeleportPosition) false false)
  (Rendering|Debug|DrawDebugLine (Transformation|GetActorLocation) (Transformation|GetWorldLocation (Variables|Default|GetTeleportpoint)) "(R=1.000000,G=0.000000,B=0.024798,A=1.000000)" 0.5 5.0)
  (bind _output_get (Variables|Default|SetTxtTPPoint (Utilities|String|Append "Boss TP Loc" " 
" (Utilities|GetDisplayName self))))
  (Rendering|Components|TextRender|SetText (Variables|Default|GetTxtPoint) (Utilities|Text|ToText(String) _output_get)))