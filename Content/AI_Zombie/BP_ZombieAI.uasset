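; Zombie enemy character that grunts at random intervals, melees the player and ragdolls on death.
; The construction script attaches per-limb, head and body collision components to skeleton sockets for locational hit detection.
; E_AttackPlayer waits briefly, then damages the player if still in range and briefly flags them as hurt.
; E_Ragdoll enables mesh physics, disables capsule collision, clears the anim class and sets IsDead, silencing grunts and new attacks.
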(event Custom|E_PlayGruntingSound
  ;[1 1 1] BeginPlay
  (if (not (Variables|Default|GetbIsDead))
    (Audio|PlaySoundatLocation "/Game/Sounds/SC_Random_Zombie_MaleGrunt.SC_Random_Zombie_MaleGrunt" (Transformation|GetActorLocation) "0, 0, 0" 1.0 1.0 0.0 0 0 0 0)))

(event Custom|E_AttackPlayer
  ;[1 1 1] DoDamage
  (if (not (Variables|Default|GetbIsDead))
    (Variables|Default|SetbIsAttacking true)
    (Utilities|FlowControl|Delay 0.5)
    (if (<= (Transformation|GetDistanceTo (Game|GetPlayerCharacter 0)) 1.5e+02)
      (bind _asbp_third_person_character (Utilities|Casting|CastToBP_ThirdPersonCharacter (Game|GetPlayerCharacter 0)))
      (Default|ETakeDamage _asbp_third_person_character)
      (Variables|/Game/ThirdPerson/Blueprints/BP_ThirdPersonCharacter.BP_ThirdPersonCharacter_C|SetbHasBeenHurt _asbp_third_person_character true)
      (Utilities|FlowControl|Delay 0.7)
      (Variables|/Game/ThirdPerson/Blueprints/BP_ThirdPersonCharacter.BP_ThirdPersonCharacter_C|SetbHasBeenHurt _asbp_third_person_character false)
      (Variables|Default|SetbIsAttacking false)
      (else
        (Variables|Default|SetbIsAttacking false)))))

(event Custom|E_Ragdoll
  ;[1 1 1] Death
  (Physics|SetSimulatePhysics (Variables|Character|GetMesh) true)
  (Collision|SetCollisionEnabled (Variables|Collision|GetCapsuleComponent) "NoCollision")
  (Variables|Default|SetAIControllerClass 0)
  (Class|SkeletalMeshComponent|SetAnimClass (Variables|Character|GetMesh))
  (Variables|Default|SetbIsDead true))

(event EventBeginPlay
  ;[1 1 1] BeginPlay
  (Utilities|Time|SetTimerbyEvent (delegate Custom|E_PlayGruntingSound) (Math|Random|RandomFloatinRange 5.0 2e+01) true))

(fn ConstructionScript
  (Utilities|FlowControl|Sequence
    (:then_0
      (Transformation|AttachComponentToComponent (Variables|Default|GetHeadCollision) (Variables|Character|GetMesh) "HeadshotPoint" "KeepWorld" "KeepWorld" "KeepWorld" true)
      (Transformation|SetRelativeLocation (Variables|Default|GetHeadCollision) "5.000000,0.000000,0.000000" false false))
    (:then_1
      (Transformation|AttachComponentToComponent (Variables|Default|GetBodyCollision) (Variables|Character|GetMesh) "spine_01" "KeepWorld" "KeepWorld" "KeepWorld" true)
      (Transformation|SetRelativeLocation (Variables|Default|GetBodyCollision) "10.000000,0.000000,0.000000" false false))
    (:then_2
      (Transformation|AttachComponentToComponent (Variables|Default|GetRightUpperArmCollision) (Variables|Character|GetMesh) "upperarm_r" "KeepWorld" "KeepWorld" "KeepWorld" true)
      (Transformation|SetRelativeLocation (Variables|Default|GetRightUpperArmCollision) "-10.000000,0.000000,-0.000000" false false))
    (:then_3
      (Transformation|AttachComponentToComponent (Variables|Default|GetRightLowerArmCollision) (Variables|Character|GetMesh) "lowerarm_r" "KeepWorld" "KeepWorld" "KeepWorld" true)
      (Transformation|SetRelativeLocation (Variables|Default|GetRightLowerArmCollision) "-25.000000,0.000000,-0.000000" false false))
    (:then_4
      (Transformation|AttachComponentToComponent (Variables|Default|GetLeftUpperArmCollision) (Variables|Character|GetMesh) "upperarm_l" "KeepWorld" "KeepWorld" "KeepWorld" true)
      (Transformation|SetRelativeLocation (Variables|Default|GetLeftUpperArmCollision) "10.000000,0.000000,-0.000000" false false))
    (:then_5
      (Transformation|AttachComponentToComponent (Variables|Default|GetLeftLowerArmCollision) (Variables|Character|GetMesh) "lowerarm_l" "KeepWorld" "KeepWorld" "KeepWorld" true)
      (Transformation|SetRelativeLocation (Variables|Default|GetLeftLowerArmCollision) "25.000000,0.000000,-0.000000" false false))
    (:then_6
      (Transformation|AttachComponentToComponent (Variables|Default|GetRightUpperLegCollision) (Variables|Character|GetMesh) "thigh_r" "KeepWorld" "KeepWorld" "KeepWorld" true)
      (Transformation|SetRelativeLocation (Variables|Default|GetRightUpperLegCollision) "25.000000,0.000000,0.000000" false false))
    (:then_7
      (Transformation|AttachComponentToComponent (Variables|Default|GetRightLowerLegCollision) (Variables|Character|GetMesh) "calf_r" "KeepWorld" "KeepWorld" "KeepWorld" true)
      (Transformation|SetRelativeLocation (Variables|Default|GetRightLowerLegCollision) "25.000000,0.000000,-0.000000" false false))
    (:then_8
      (Transformation|AttachComponentToComponent (Variables|Default|GetLeftUpperLegCollision) (Variables|Character|GetMesh) "thigh_l" "KeepWorld" "KeepWorld" "KeepWorld" true)
      (Transformation|SetRelativeLocation (Variables|Default|GetLeftUpperLegCollision) "-25.000000,0.000000,0.000000" false false))
    (:then_9
      (Transformation|AttachComponentToComponent (Variables|Default|GetLeftLowerLegCollision) (Variables|Character|GetMesh) "calf_l" "KeepWorld" "KeepWorld" "KeepWorld" true)
      (Transformation|SetRelativeLocation (Variables|Default|GetLeftLowerLegCollision) "-25.000000,0.000000,-0.000000" false false))))