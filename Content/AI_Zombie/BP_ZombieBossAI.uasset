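; Zombie boss AI Blueprint that adds movement sounds and a melee attack for the boss.
; On BeginPlay it checks IsRunning and starts a looping timer that plays random run or walk sounds at its location, faster when running.
; AttackMelee plays a standing right-hand attack animation directly on the mesh and returns MeleeRate.
; SetWeapon is left empty.
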(event Custom|E_PlayWalkSound
  (Audio|PlaySoundatLocation "/Game/Sounds/SC_Random_Boss_Walk.SC_Random_Boss_Walk" (Transformation|GetActorLocation) "0, 0, 0" 1.0 1.0 0.0 0 0 0 0))

(event Custom|E_PlayRunSound
  (Audio|PlaySoundatLocation "/Game/Sounds/SC_Random_Boss_Run.SC_Random_Boss_Run" (Transformation|GetActorLocation) "0, 0, 0" 1.0 1.0 0.0 0 0 0 0))

(event EventBeginPlay
  (if (Variables|Default|GetbIsRunning)
    (Utilities|Time|SetTimerbyEvent (delegate Custom|E_PlayRunSound) 0.5 true)
    (else
      (Utilities|Time|SetTimerbyEvent (delegate Custom|E_PlayWalkSound) 1.0 true))))

(fn ConstructionScript)

(fn AttackMelee
  (Components|Animation|PlayAnimation (Variables|Character|GetMesh) "/Game/AI_Zombie/BSP_ZombieAnims/Animations/Standing/Attack/AS_NAAT_Zombie_Attack_RH_Stand.AS_NAAT_Zombie_Attack_RH_Stand" false)
  (return (Variables|Default|GetMeleeRate)))

(fn SetWeapon
  (params (CombatType :type Byte :default 0)))