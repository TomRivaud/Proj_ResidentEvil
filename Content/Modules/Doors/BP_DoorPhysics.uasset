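; Physics-driven door that is either open or locked behind one requirement: key, fingerprint, sample, fuse or keycard.
; Lock flags set its initial state, label text and nav area; closed doors lock the constraint swing and show interact prompts when the player is near.
; Lock checks go to BP_ThirdPersonGameMode; opening frees the swing, restores navigation and plays a sound.
; Tick disables door collision while rotated over 70 degrees from its starting rotation.
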(event OnComponentBeginOverlap(SphereCol)
  (params (OverlappedComponent :type Primitive%20Component%20Object%20Reference) (OtherActor :type Actor%20Object%20Reference) (OtherComp :type Primitive%20Component%20Object%20Reference) (OtherBodyIndex :type Integer) (bFromSweep :type Boolean) (SweepResult :type Hit%20Result%20Structure%20%28by%20ref%29))
  (if (Actor|ActorHasTag OtherActor "Player")
    (if (not (Variables|Default|GetbIsOpen))
      (Rendering|SetVisibility (Variables|Default|GetInteractFace) true false))))

(event OnComponentEndOverlap(SphereCol)
  (params (OverlappedComponent :type Primitive%20Component%20Object%20Reference) (OtherActor :type Actor%20Object%20Reference) (OtherComp :type Primitive%20Component%20Object%20Reference) (OtherBodyIndex :type Integer))
  (if (Actor|ActorHasTag OtherActor "Player")
    (if (not (Variables|Default|GetbIsOpen))
      (Rendering|SetVisibility (Variables|Default|GetInteractFace) false false))))

(event Custom|E_OpenDoor
  (Variables|Default|SetbIsOpen true)
  (Class|NavModifierComponent|SetAreaClass (Variables|Default|GetNavModifier) "/Script/NavigationSystem.NavArea_Default")
  (Class|PhysicsConstraintComponent|SetAngularSwing1Limit (Variables|Default|GetPhysicsConstraint) "ACM_Limited" 9e+01)
  (CallFunction|SetText)
  (CallFunction|EPlaySoundDoorOpening)
  (Rendering|SetVisibility (Variables|Default|GetInteractFace) false false))

(event Custom|E_CheckDoor
  (if (Variables|Default|GetLockedByKey01)
    (Default|ECheckKeydoor01 (Variables|Default|GetAs%20BP%20Third%20Person%20Game%20Mode) self)
    (elif (Variables|Default|GetLockedByHand)
      (Default|ECheckHand (Variables|Default|GetAs%20BP%20Third%20Person%20Game%20Mode) self)
      (elif (Variables|Default|GetLockedBySample)
        (Default|ECheckSample (Variables|Default|GetAs%20BP%20Third%20Person%20Game%20Mode) self)
        (elif (Variables|Default|GetLockedByFuse)
          (Default|ECheckFuse (Variables|Default|GetAs%20BP%20Third%20Person%20Game%20Mode) self)
          (elif (Variables|Default|GetLockedByKeycard)
            (Default|ECheckKeycard (Variables|Default|GetAs%20BP%20Third%20Person%20Game%20Mode) self)))))))

(event Custom|E_PlaySoundDoorOpening
  (Audio|PlaySoundatLocation "/Game/Sounds/SC_DoorOpening.SC_DoorOpening" (Transformation|GetActorLocation) "0, 0, 0" 1.0 1.0 0.0 0 0 0 0))

(event EventTick
  (params (DeltaSeconds :type Float%20%28single-precision%29))
  (bind _baserelativerot (Variables|Default|GetBaseRelativeRot))
  (bind _sm_door (Variables|Default|GetSM_Door))
  (bind _relativerotation (Variables|/Script/Engine.SceneComponent|GetRelativeRotation _sm_door))
  (bind _returnvalue (- (.yaw _relativerotation) (.yaw _baserelativerot)))
  (bind _returnvalue_2 (- (.pitch _relativerotation) (.pitch _baserelativerot)))
  (bind _returnvalue_3 (- (.roll _relativerotation) (.roll _baserelativerot)))
  (if (Math|Boolean|ORBoolean (or (> _returnvalue_3 7e+01) (< _returnvalue_3 -7e+01)) (or (> _returnvalue_2 7e+01) (< _returnvalue_2 -7e+01)) (or (> _returnvalue 7e+01) (< _returnvalue -7e+01)))
    (Collision|SetCollisionResponsetoAllChannels (Variables|Default|GetSM_Door) "ECR_Ignore")
    (else
      (Collision|SetCollisionResponsetoAllChannels (Variables|Default|GetSM_Door) "ECR_Block"))))

(event EventBeginPlay
  (bind _physicsconstraint (Variables|Default|GetPhysicsConstraint))
  (bind _asbp_third_person_game_mode (Utilities|Casting|CastToBP_ThirdPersonGameMode (Game|GetGameMode)))
  (Variables|Default|SetAs%20BP%20Third%20Person%20Game%20Mode _asbp_third_person_game_mode)
  (Variables|Default|SetBaseRelativeRot (Variables|/Script/Engine.SceneComponent|GetRelativeRotation (Variables|Default|GetSM_Door)))
  (if (Variables|Default|GetbIsOpen)
    (Class|PhysicsConstraintComponent|SetAngularSwing1Limit _physicsconstraint "ACM_Limited" 9e+01)
    (else
      (Class|PhysicsConstraintComponent|SetAngularSwing1Limit _physicsconstraint "ACM_Locked" 0.0))))

(fn ConstructionScript
  (if (Math|Boolean|ORBoolean (Variables|Default|GetLockedByKey01) (Variables|Default|GetLockedByHand) (Variables|Default|GetLockedBySample) (Variables|Default|GetLockedByFuse) (Variables|Default|GetLockedByKeycard))
    (Variables|Default|SetbIsOpen false)
    (Class|NavModifierComponent|SetAreaClass (Variables|Default|GetNavModifier) "/Script/NavigationSystem.NavArea_Null")
    (else
      (Variables|Default|SetbIsOpen true)
      (Class|NavModifierComponent|SetAreaClass (Variables|Default|GetNavModifier) "/Script/NavigationSystem.NavArea_Default")))
  (Components|StaticMesh|SetStaticMesh (Variables|Default|GetSM_Door) (Variables|Default|GetDoorMesh))
  (CallFunction|SetText))

(fn SetText
  (if (Variables|Default|GetbIsOpen)
    (Variables|Default|SetDoorState "Opened")
    (Rendering|Components|TextRender|SetText (Variables|Default|GetTextRender) (Utilities|Text|ToText(String) (Variables|Default|GetDoorState)))
    (else
      (Variables|Default|SetDoorState "Closed")
      (if (Variables|Default|GetLockedByKey01)
        (Variables|Default|SetLockedBy "Key01")
        (Rendering|Components|TextRender|SetText (Variables|Default|GetTextRender) (Utilities|Text|ToText(String) (Utilities|String|Append (Variables|Default|GetDoorState) " 
" "Need: " (Variables|Default|GetLockedBy))) :!label _label)
        (elif (Variables|Default|GetLockedByHand)
          (Variables|Default|SetLockedBy "Fingerprint")
          (goto _label)
          (elif (Variables|Default|GetLockedBySample)
            (Variables|Default|SetLockedBy "Sample")
            (goto _label)
            (elif (Variables|Default|GetLockedByFuse)
              (Variables|Default|SetLockedBy "Fuse")
              (goto _label)
              (elif (Variables|Default|GetLockedByKeycard)
                (Variables|Default|SetLockedBy "Keycard")
                (goto _label)))))))))