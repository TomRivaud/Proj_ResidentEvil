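; Modular glass wall actor Blueprint that lets each placed instance pick one of three wall variants.
; The construction script switches on the ENWallGlass enum to set SMWallGlass to the full, large-border or small-border glass mesh.
; Every variant applies the same materials, with glass on the second slot and white prototype grid on the others.
; The event graph holds only disabled placeholder events, so the actor has no runtime logic.
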(event EventBeginPlay)

(event Collision|EventActorBeginOverlap
  (params (OtherActor :type Actor%20Object%20Reference)))

(event EventTick
  (params (DeltaSeconds :type Float%20%28single-precision%29)))

(fn ConstructionScript
  (bind _sm_wall_glass (Variables|Default|GetSM_Wall_Glass))
  (bind _sm_wall_glass_2 (Variables|Default|GetSM_Wall_Glass))
  (bind _sm_wall_glass_3 (Variables|Default|GetSM_Wall_Glass))
  (switch Utilities|FlowControl|Switch|SwitchonEN_WallGlass (Variables|Default|GetEN_WallGlass)
    (:NewEnumerator0
      (Components|StaticMesh|SetStaticMesh _sm_wall_glass_2 "/Game/Modules/Glasses/SM_Wall_Glass_Full.SM_Wall_Glass_Full")
      (Rendering|Material|SetMaterial _sm_wall_glass_2 0 "/Game/MaterialsVFX/ProtoMat/MI_PrototypeGrid_White.MI_PrototypeGrid_White")
      (Rendering|Material|SetMaterial _sm_wall_glass_2 1 "/Game/ScienceLab/Materials/Rooms/Wall/MI_Glass02.MI_Glass02")
      (Rendering|Material|SetMaterial _sm_wall_glass_2 2 "/Game/MaterialsVFX/ProtoMat/MI_PrototypeGrid_White.MI_PrototypeGrid_White")
      (Rendering|Material|SetMaterial _sm_wall_glass_2 3 "/Game/MaterialsVFX/ProtoMat/MI_PrototypeGrid_White.MI_PrototypeGrid_White"))
    (:NewEnumerator2
      (Components|StaticMesh|SetStaticMesh _sm_wall_glass "/Game/Modules/Glasses/SM_Wall_Glass_Large.SM_Wall_Glass_Large")
      (Rendering|Material|SetMaterial _sm_wall_glass 0 "/Game/MaterialsVFX/ProtoMat/MI_PrototypeGrid_White.MI_PrototypeGrid_White")
      (Rendering|Material|SetMaterial _sm_wall_glass 1 "/Game/ScienceLab/Materials/Rooms/Wall/MI_Glass02.MI_Glass02")
      (Rendering|Material|SetMaterial _sm_wall_glass 2 "/Game/MaterialsVFX/ProtoMat/MI_PrototypeGrid_White.MI_PrototypeGrid_White")
      (Rendering|Material|SetMaterial _sm_wall_glass 3 "/Game/MaterialsVFX/ProtoMat/MI_PrototypeGrid_White.MI_PrototypeGrid_White"))
    (:NewEnumerator3
      (Components|StaticMesh|SetStaticMesh _sm_wall_glass_3 "/Game/Modules/Glasses/SM_Wall_Glass_Small.SM_Wall_Glass_Small")
      (Rendering|Material|SetMaterial _sm_wall_glass_3 0 "/Game/MaterialsVFX/ProtoMat/MI_PrototypeGrid_White.MI_PrototypeGrid_White")
      (Rendering|Material|SetMaterial _sm_wall_glass_3 1 "/Game/ScienceLab/Materials/Rooms/Wall/MI_Glass02.MI_Glass02")
      (Rendering|Material|SetMaterial _sm_wall_glass_3 2 "/Game/MaterialsVFX/ProtoMat/MI_PrototypeGrid_White.MI_PrototypeGrid_White")
      (Rendering|Material|SetMaterial _sm_wall_glass_3 3 "/Game/MaterialsVFX/ProtoMat/MI_PrototypeGrid_White.MI_PrototypeGrid_White"))))