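; NPC character Blueprint that fights as melee or ranged, with CombatType setting its mesh material and rifle.
; BeginPlay removes the melee rifle, speeds up rush-controller NPCs and resets location after a delay.
; Events set or clear combat flags from the Blackboard CombatState, while functions play attack animations and return attack rates.
; E_Ragdoll enables mesh physics, disables capsule collision and clears the animation and AI controller classes.
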(event Custom|WeaponCheck
  (switch Utilities|FlowControl|Switch|SwitchonEN_CombatState (Utilities|Enum|ByteToEnumEN_CombatState (Class|BlackboardComponent|GetValueasEnum (AI|GetBlackboard 0) (Utilities|Name|MakeLiteralName "CombatState")))
    (:NewEnumerator0
      (Variables|Default|SetMeleeCombat true)
      (if (Variables|Default|GetRangedCombat)
        _))
    (:NewEnumerator1
      (Variables|Default|SetRangedCombat true)
      (if (Variables|Default|GetMeleeCombat)
        _))))

(event Custom|ResetCombat
  (switch Utilities|FlowControl|Switch|SwitchonEN_CombatState (Utilities|Enum|ByteToEnumEN_CombatState (Class|BlackboardComponent|GetValueasEnum (AI|GetBlackboard 0) (Utilities|Name|MakeLiteralName "CombatState")))
    (:NewEnumerator0
      _)
    (:NewEnumerator1
      _))
  (Variables|Default|SetMeleeCombat false)
  (Variables|Default|SetRangedCombat false)
  (AI|Components|Blackboard|SetValueasEnum (AI|GetBlackboard 0) (Utilities|Name|MakeLiteralName "CombatState"))
  (AI|Components|Blackboard|SetValueasEnum (AI|GetBlackboard 0) (Utilities|Name|MakeLiteralName "BaseState")))

(event Custom|E_Ragdoll
  (Physics|SetSimulatePhysics (Variables|Character|GetMesh) true)
  (Collision|SetCollisionEnabled (Variables|Collision|GetCapsuleComponent) "NoCollision")
  (Variables|Default|SetAIControllerClass 0)
  (Class|SkeletalMeshComponent|SetAnimClass (Variables|Character|GetMesh)))

(event EventBeginPlay
  (Variables|Default|SetActorLoc (Transformation|GetActorLocation))
  (Utilities|FlowControl|Sequence
    (:then_0
      (switch Utilities|FlowControl|Switch|SwitchonEN_CombatState (Variables|Default|GetCombatType)
        (:NewEnumerator0
          (Components|DestroyComponent (Variables|Default|GetRifle))
          (switch Utilities|FlowControl|Switch|SwitchonEN_CombatState (Variables|Default|GetCombatType)
            (:NewEnumerator0
              (Variables|Default|SetMeleeCombat true)
              (Rendering|Material|SetMaterial (Variables|Character|GetMesh) 0 "/Game/NPC/Anim/Materials/Beta_HighLimbsGeoSG_Blue.Beta_HighLimbsGeoSG_Blue"))
            (:NewEnumerator1
              (Variables|Default|SetRangedCombat true))))))
    (:then_1
      (if (== (AI|GetAIController 0) "/Game/NPC/AI_NPCRush.AI_NPCRush")
        (Variables|/Script/Engine.CharacterMovementComponent|SetMaxWalkSpeed (Variables|Character|GetCharacterMovement) 7e+02)
        (Development|PrintString "Hello")))
    (:then_2
      (Utilities|FlowControl|Delay 5.0)
      (Transformation|SetActorLocation (Variables|Default|GetActorLoc) false false))))

(fn ConstructionScript
  (switch Utilities|FlowControl|Switch|SwitchonEN_CombatState (Variables|Default|GetCombatType)
    (:NewEnumerator0
      (Rendering|Material|SetMaterial (Variables|Character|GetMesh) 0 "/Game/NPC/Anim/Materials/Beta_HighLimbsGeoSG_Blue.Beta_HighLimbsGeoSG_Blue")
      (Rendering|SetVisibility (Variables|Default|GetRifle) false false))
    (:NewEnumerator1
      (Rendering|Material|SetMaterial (Variables|Character|GetMesh) 0 "/Game/NPC/Anim/Materials/Beta_HighLimbsGeoSG_Red.Beta_HighLimbsGeoSG_Red")
      (Rendering|SetVisibility (Variables|Default|GetRifle) true false))))

(fn FireRifle
  (Components|Animation|PlayAnimation (Variables|Character|GetMesh) "/Game/NPC/Anim/Firing_Rifle.Firing_Rifle" false)
  (return (Variables|Default|GetFireRate)))

(fn AttackMelee
  (Components|Animation|PlayAnimation (Variables|Character|GetMesh) "/Game/NPC/Anim/Melee_Smash.Melee_Smash" false)
  (return (Variables|Default|GetMeleeRate)))

(fn SetWeapon
  (params (CombatType :type EN_CombatState%20Enum :default "NewEnumerator2"))
  (switch Utilities|FlowControl|Switch|SwitchonEN_CombatState CombatType
    (:NewEnumerator0
      (Components|DestroyComponent (Variables|Default|GetRifle))
      (switch Utilities|FlowControl|Switch|SwitchonEN_CombatState CombatType
        (:NewEnumerator0
          (Variables|Default|SetMeleeCombat true))
        (:NewEnumerator1
          (Variables|Default|SetRangedCombat true))))))